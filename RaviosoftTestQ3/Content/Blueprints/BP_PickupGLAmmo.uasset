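; BP_PickupGLAmmo is a grenade launcher ammo pickup that is consumed when an SPawn overlaps it.
; It only works if the pawn holds a valid gun whose ShootType is Projectile; otherwise the pickup stays in place.
; On pickup it adds a fixed amount to TotalGLAmmo, copies that total into CurrentAmmo, plays a 2D pickup sound and destroys itself.
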(event `self.ReceiveActorBeginOverlap`
  (params (OtherActor :type "Actor Object Reference"))
  (bind _asspawn (cast `SPawn` OtherActor))
  (bind _currentgun (`SPawn.CurrentGun` _asspawn))
  (`/Engine/EditorBlueprintResources/StandardMacros.IsValid` _currentgun
    (:`Is Valid`
      (switch `EShootType` (`Gun.ShootType` _currentgun)
        (:`Projectile`
          (bind _output_get (set `SPawn.TotalGLAmmo` (+ (`SPawn.TotalGLAmmo` _asspawn) 20) _asspawn))
          (set `SPawn.CurrentAmmo` _output_get _asspawn)
          (`GameplayStatics.SpawnSound2D` "/Game/PrototypeWeap/Sound/Pistol/Pistol_AmmoPickup_Cue.Pistol_AmmoPickup_Cue" 1.0 1.0 0.0 null)
          (`self.K2_DestroyActor`))))))

(fn `UserConstructionScript`)