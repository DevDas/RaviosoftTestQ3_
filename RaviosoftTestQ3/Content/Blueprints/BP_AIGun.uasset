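; BP_AIGun is an AI gun turret with base, turret and pipe meshes, a health component and a health widget.
; On BeginPlay it caches the player's SPawn and sets itself as the WBP_Health widget's owner.
; When HealthComp reports death, it adds a random bonus to the player's score and calls DeadEffects.
; DeadEffects applies the dead material to all three meshes and spawns an explosion particle and sound.
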(event `self.ReceiveBeginPlay`
  (bind _asspawn (cast `SPawn` (`GameplayStatics.GetPlayerPawn` 0)))
  (set `self.As SPawn` _asspawn)
  (bind _aswbp_health (cast `/Game/Blueprints/WBP_Health` (`WidgetComponent.GetWidget` (`self.Widget`))))
  (set `/Game/Blueprints/WBP_Health.Owner` self _aswbp_health))

(event `self.ReceiveTick`
  (params (DeltaSeconds :type "Float (single-precision)")))

(event `self.HealthComp.OnDeath`
  (bind _as_spawn (`self.As SPawn`))
  (set `SPawn.Score` (+ (`SPawn.Score` _as_spawn) (`KismetMathLibrary.RandomIntegerInRange` 15 25)) _as_spawn)
  (`self.DeadEffects`))

(fn `DeadEffects`
  (bind (_returnvalue_location _returnvalue_rotation _returnvalue_scale) (`KismetMathLibrary.BreakTransform` (`self.GetTransform`)))
  (`PrimitiveComponent.SetMaterial` (`self.BaseMesh`) 0 "/Game/Assets/M_Dead.M_Dead")
  (`PrimitiveComponent.SetMaterial` (`self.TurretMesh`) 0 "/Game/Assets/M_Dead.M_Dead")
  (`PrimitiveComponent.SetMaterial` (`self.TurretPipe`) 0 "/Game/Assets/M_Dead.M_Dead")
  (`GameplayStatics.SpawnEmitterAtLocation` "/Game/PrototypeWeap/FX/P_RocketLauncher_Explosion.P_RocketLauncher_Explosion" _returnvalue_location _returnvalue_rotation _returnvalue_scale)
  (`GameplayStatics.SpawnSoundAtLocation` "/Game/PrototypeWeap/Sound/GrenadeLauncher/GL_Explosion_Cue.GL_Explosion_Cue" _returnvalue_location (struct) 1.0 1.0 0.0 null null))

(fn `UserConstructionScript`)