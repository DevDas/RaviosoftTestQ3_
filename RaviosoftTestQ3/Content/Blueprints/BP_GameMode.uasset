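; Game mode that handles the win condition: the player wins when no AIGun enemies remain.
; BeginPlay counts all AIGun actors into TotalEnemyLeft and prints it; nothing in this file decrements that count.
; Tick polls the count and, once it reaches zero, sets GameOver, replaces all widgets with WBP_Won, and switches to UI-only input with a visible cursor.
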(event `self.ReceiveBeginPlay`
  (bind _outactors (`GameplayStatics.GetAllActorsOfClass` "/Script/RaviosoftTestQ3.AIGun"))
  (bind _output_get (set `self.TotalEnemyLeft` (`KismetArrayLibrary.Array_Length` _outactors)))
  (`KismetSystemLibrary.PrintString` (`KismetStringLibrary.Conv_IntToString` _output_get)))

(event `self.ReceiveTick`
  (params (DeltaSeconds :type "Float (single-precision)"))
  (bind _returnvalue (`GameplayStatics.GetPlayerController` 0))
  (if (`self.GameOver`)
    _
    (elif (<= (`self.TotalEnemyLeft`) 0)
      (set `self.GameOver` true)
      (`WidgetLayoutLibrary.RemoveAllWidgets`)
      (bind _returnvalue_2 (`|CreateWidget` "/Game/Blueprints/WBP_Won.WBP_Won_C"))
      (`UserWidget.AddToViewport` _returnvalue_2 0)
      (`WidgetBlueprintLibrary.SetInputMode_UIOnlyEx` _returnvalue _returnvalue_2)
      (set `PlayerController.bShowMouseCursor` true _returnvalue))))

(fn `UserConstructionScript`)